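; BP_ParkourCharacter is an auto-running character that moves constantly along world -Y and can switch between 2D and 3D cameras.
; BeginPlay attaches a sword, a FlipFlop on SwitchViews (temporarily bound to Backspace) swaps cameras, and Tick picks the sprint effect from IsIn2DMode.
; DealDamage decrements Health until Death ragdolls the mesh and loads DefeatLevel.
; Separate events load Victory and briefly flash a portal effect widget.
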(event Custom|SwitchViews
  ;[0.15 0.02576 0.1084 0.5] Temporary Setup For Switching Perspectives Using Backspace Key
  ;;[0.15 0.15 0.15 0.5] Can be Called Elsewhere
  (Utilities|FlowControl|FlipFlop
    (:A
      (Components|Activation|SetActive (Variables|Default|GetCameraFor2D) true false)
      (Components|Activation|SetActive (Variables|Default|GetCameraFor3D) false false))
    (:B
      (Components|Activation|SetActive (Variables|Default|GetCameraFor2D) false false)
      (Components|Activation|SetActive (Variables|Default|GetCameraFor3D) true false))))

(event Custom|Death
  ;[0.15 0.15 0.15 0.5] Death
  ;;[0.15 0.15 0.15 0.5] ragdoll
  (Physics|SetSimulatePhysics (Variables|Character|GetMesh) true)
  ;;[0.15 0.15 0.15 0.5] Delay
  (Utilities|FlowControl|Delay 0.11)
  ;;[0.15 0.15 0.15 0.5] Death Sound
  (Audio|PlaySound2D "/Game/MyProject/Audio/Cat/Crunch.Crunch" 1.0 1.0 0.0 0 0)
  ;;[0.15 0.15 0.15 0.5] Game Over UI
  (Game|OpenLevel(byName) "DefeatLevel"))

(event Custom|Victory
  (Game|OpenLevel(byName) "Victory"))

(event Custom|DealDamage
  (bind _health (Variables|Default|GetHealth))
  (Math|Integer|DecrementInt _health
    (:%20%20
      (if (< _health 1)
        (CallFunction|Death)
        (else
          (Audio|PlaySound2D "/Game/MyProject/Audio/Cat/Crunch.Crunch" 0.5 1.25 0.0 0 0))))))

(event Custom|CreatePortalWidget
  (bind _returnvalue (UserInterface|CreateWidget "/Game/MyProject/UI/UI_Portal_Effect.UI_Portal_Effect_C" (Game|GetPlayerController 0)))
  (UserInterface|Viewport|AddtoViewport _returnvalue 0)
  (Widget|SetVisibility _returnvalue "Visible")
  (Utilities|FlowControl|Delay 0.3)
  (Widget|SetVisibility _returnvalue "Hidden")
  (Widget|SetVisibility _returnvalue "Collapsed")
  (Widget|RemovefromParent _returnvalue))

(event EventBeginPlay
  (bind _mesh (Variables|Character|GetMesh))
  (bind _returnvalue (Game|SpawnActorfromClass "/Game/MyProject/Meshes/BP_Sword.BP_Sword_C" (Transformation|GetSocketTransform _mesh "SwordSocket" "RTS_World") "Undefined" "MultiplyWithRoot" 0 0))
  (Transformation|AttachComponentToComponent _returnvalue _mesh "SwordSocket" "SnapToTarget" "SnapToTarget" "SnapToTarget" true))

(event Collision|EventActorBeginOverlap
  (params (OtherActor :type Actor%20Object%20Reference)))

(event EventTick
  (params (DeltaSeconds :type Float%20%28single-precision%29))
  ;[0.15 0.15 0.15 0.5] Move Player forward on Event Tick
  (Pawn|Input|AddMovementInput "0.000000,-1.000000,0.000000" 1.0 false)
  (if (Variables|Default|GetbIsIn2DMode)
    (Components|Activation|SetActive (Variables|Default|GetNS_Sprint2D) true false)
    (Components|Activation|SetActive (Variables|Default|GetNS_Sprint_3D) false false)
    (else
      (Components|Activation|SetActive (Variables|Default|GetNS_Sprint2D) false false)
      (Components|Activation|SetActive (Variables|Default|GetNS_Sprint_3D) true false))))

(event Input|KeyboardEvents|Backspace
  (params (Key :type Key%20Structure :default "None"))
  ;[0.15 0.02576 0.1084 0.5] Temporary Setup For Switching Perspectives Using Backspace Key
  (:Pressed
    (CallFunction|SwitchViews)))

(fn ConstructionScript)