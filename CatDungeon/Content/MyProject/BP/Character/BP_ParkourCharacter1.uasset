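; Parkour character Blueprint that runs automatically and can switch between 2D and 3D camera views.
; Tick applies constant movement input along world negative Y.
; The SwitchViews event uses a FlipFlop to toggle the active camera, temporarily bound to Backspace and callable from elsewhere.
; The Death event is a stub that only prints a debug string and waits briefly, and the IsIn2DMode variable is unused.
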(event Custom|SwitchViews
  ;[0.15 0.02576 0.1084 0.5] Temporary Setup For Switching Perspectives Using Backspace Key
  ;;[0.15 0.15 0.15 0.5] Can be Called Elsewhere
  (Utilities|FlowControl|FlipFlop
    (:A
      (Components|Activation|SetActive (Variables|Default|GetCameraFor2D) true false)
      (Components|Activation|SetActive (Variables|Default|GetCameraFor3D) false false))
    (:B
      (Components|Activation|SetActive (Variables|Default|GetCameraFor2D) false false)
      (Components|Activation|SetActive (Variables|Default|GetCameraFor3D) true false))))

(event Custom|Death
  ;[0.15 0.15 0.15 0.5] Death
  (Development|PrintString "Hello")
  (Utilities|FlowControl|Delay 0.8))

(event EventBeginPlay)

(event Collision|EventActorBeginOverlap
  (params (OtherActor :type Actor%20Object%20Reference)))

(event EventTick
  (params (DeltaSeconds :type Float%20%28single-precision%29))
  ;[0.15 0.15 0.15 0.5] Move Player forward on Event Tick
  (Pawn|Input|AddMovementInput "0.000000,-1.000000,0.000000" 1.0 false))

(event Input|KeyboardEvents|Backspace
  (params (Key :type Key%20Structure :default "None"))
  ;[0.15 0.02576 0.1084 0.5] Temporary Setup For Switching Perspectives Using Backspace Key
  (:Pressed
    (CallFunction|SwitchViews)))

(fn ConstructionScript)